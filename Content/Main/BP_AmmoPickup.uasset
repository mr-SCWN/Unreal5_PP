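; BP_AmmoPickup is an ammo pickup that a Lab1Character collects by overlapping its SphereCollision.
; The overlap adds Amount to the character's CurrentAmmo, clamped to MaxAmmo, then destroys the pickup and prints the new ammo count.
; On BeginPlay, it sets the Sphere component's relative height to half its local bounds height plus a fixed offset.
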(event OnComponentBeginOverlap(SphereCollision)
  (params (OverlappedComponent :type Primitive%20Component%20Object%20Reference) (OtherActor :type Actor%20Object%20Reference) (OtherComp :type Primitive%20Component%20Object%20Reference) (OtherBodyIndex :type Integer) (bFromSweep :type Boolean) (SweepResult :type Hit%20Result%20Structure%20%28by%20ref%29))
  (bind _aslab_1character (Utilities|Casting|CastToLab1Character OtherActor))
  (bind _output_get (Variables|/Game/Main/Lab1Character.Lab1Character_C|SetCurrentAmmo _aslab_1character (Math|Integer|Min(Integer) (+ (Variables|/Game/Main/Lab1Character.Lab1Character_C|GetCurrentAmmo _aslab_1character) (Variables|Default|GetAmount)) (Variables|/Game/Main/Lab1Character.Lab1Character_C|GetMaxAmmo _aslab_1character))))
  (Actor|DestroyActor)
  (Development|PrintString (Utilities|String|Append "Ammo restored, shots left: " (Utilities|String|ToString(Integer) _output_get))))

(event EventBeginPlay
  (bind _sphere (Variables|Default|GetSphere))
  (bind (_min _max) (Components|StaticMesh|GetLocalBounds _sphere))
  (Transformation|SetRelativeLocation (Variables|Default|GetSphere) (Math|Vector|MakeVector 0.0 0.0 (+ (/ (- (.Z (Math|Vector|BreakVector _max)) (.Z (Math|Vector|BreakVector _min))) 2.0) 1e+02)) false false))

(event Collision|EventActorBeginOverlap
  (params (OtherActor :type Actor%20Object%20Reference)))

(event EventTick
  (params (DeltaSeconds :type Float%20%28single-precision%29)))

(fn ConstructionScript)